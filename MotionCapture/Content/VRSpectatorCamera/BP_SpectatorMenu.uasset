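; Actor for the VR spectator camera's menu, showing a widget that is operated by mouse through a fake cursor.
; EnableMenu and DisableMenu toggle input, tick, cursor mesh and widget visibility, with the menu enabled on BeginPlay.
; Each tick, input axes slide the WidgetInteraction component, which is nudged back toward center when off the widget.
; The CameraMenuInteract action presses and releases a simulated left mouse button on the widget.
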(event `self.ReceiveBeginPlay`
  ;[1 0 0] BEGIN PLAY
  ;[0.5 0 1] Remember to always call the parent event if you don't want to override
  (`parent.ReceiveBeginPlay`)
  (`self.EnableMenu`))

(event `self.ReceiveTick`
  (params (DeltaSeconds :type "Float (single-precision)"))
  (bind (_returnvalue_x _returnvalue_y _returnvalue_z) (`KismetMathLibrary.BreakVector` (`KismetMathLibrary.NegateVector` (* (`KismetMathLibrary.Normal` (`SceneComponent.RelativeLocation` (`self.WidgetInteraction`))) (`self.NudgeDeltaMultiplier`)))))
  ;[1 0 0] TICK
  ;[1 1 1] If we are interacting with the widget, move our "fake mouse"
  (`self.MoveWidgetInteraction`)
  (if (not (`WidgetInteractionComponent.IsOverHitTestVisibleWidget` (`self.WidgetInteraction`)))
    ;[1 1 1] If not, move our fake mouse towards the center of the widget
    (`SceneComponent.K2_AddRelativeLocation` (`self.WidgetInteraction`) (`KismetMathLibrary.MakeVector` 0.0 _returnvalue_y _returnvalue_z) false false)))

(event `InputAction|CameraMenuInteract`
  (params (Key :type "Key Structure"))
  (bind _widgetinteraction (`self.WidgetInteraction`))
  ;[1 1 1] Menu Interact Input
  (:`Pressed`
    (`WidgetInteractionComponent.PressPointerKey` _widgetinteraction "LeftMouseButton"))
  (:`Released`
    (`WidgetInteractionComponent.ReleasePointerKey` _widgetinteraction "LeftMouseButton")))

(fn `DisableMenu`
  (set `self.bMenuEnabled` false)
  (`self.DisableInput` (`GameplayStatics.GetPlayerController` 0))
  (`self.SetActorTickEnabled` false)
  (`self.SetCursorVisibility` false)
  (`self.SetWidgetVisibility` false))

(fn `EnableMenu`
  (`self.VRSpectatorMenu`
    (:`then`
      (`self.SetWidgetVisibility` true))
    (:`else`
      ;[1 1 1] Create Widget Blueprint if none exists
      (bind _returnvalue (`|CreateWidget` "/MotionCapture/VRSpectatorCamera/WBP_VRSpectatorMenu.WBP_VRSpectatorMenu_C" (`GameplayStatics.GetPlayerController` 0)))
      (set `self.VRSpectatorMenu` _returnvalue)))
  ;[1 1 1] This will force the mouse cursor to lock on the window
  (`WidgetBlueprintLibrary.SetInputMode_GameOnly` (`GameplayStatics.GetPlayerController` 0))
  ;[1 1 1] Enable input for mouse axis values
  (`self.EnableInput` (`GameplayStatics.GetPlayerController` 0))
  (`self.SetActorTickEnabled` true)
  (`self.SetCursorVisibility` true)
  (set `self.bMenuEnabled` true))

(fn `InputAxisModifier`
  (params (AxisValue :type "Float (double-precision)"))
  (returns (ReturnValue :type "Float (double-precision)"))
  (return (* AxisValue (`self.InputAxisMultiplier`))))

(fn `MoveWidgetInteraction`
  (`SceneComponent.K2_AddRelativeLocation` (`self.WidgetInteraction`) (`KismetMathLibrary.MakeVector` 0.0 (`self.InputAxisModifier` (* (`self.GetInputAxisValue`) -1.0)) (`self.InputAxisModifier` (`self.GetInputAxisKeyValue`))) false false))

(fn `SetCursorVisibility`
  (params (bNewVisibility :type Boolean))
  (`SceneComponent.SetVisibility` (`self.StaticMeshCursor`) bNewVisibility false))

(fn `SetWidgetVisibility`
  (params (bNewVisibility :type Boolean))
  (`SceneComponent.SetVisibility` (`self.Widget`) bNewVisibility false))

(fn `UserConstructionScript`)