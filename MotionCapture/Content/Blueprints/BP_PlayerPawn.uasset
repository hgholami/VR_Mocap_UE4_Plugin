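; BP_PlayerPawn is a VR player pawn with smooth thumbstick locomotion and an IK-driven body.
; On BeginPlay, when an HMD is enabled, it sets floor-level tracking origin and enables input.
; Left-stick axes add movement along the camera's forward and right vectors, flattened to horizontal without renormalizing and scaled by MovementSpeed.
; The construction script hands the skeletal mesh, camera and both motion controllers to the IKBody component.
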(event `self.ReceiveBeginPlay`
  ;[1 1 1] BEGIN PLAY
  (if (`HeadMountedDisplayFunctionLibrary.IsHeadMountedDisplayEnabled`)
    (`HeadMountedDisplayFunctionLibrary.SetTrackingOrigin` "Floor")
    (`self.EnableInput` (`GameplayStatics.GetPlayerController` 0))))

(event `InputAxis|MovementAxisLeft_X`
  (params (AxisValue :type "Float (single-precision)"))
  (bind (_returnvalue_x _returnvalue_y) (`KismetMathLibrary.BreakVector` (`SceneComponent.GetRightVector` (`self.Camera`))))
  ;[1 1 1] Advanced Locomotion
  (if (not (== AxisValue 0.0))
    (`self.AddMovementInput` (`KismetMathLibrary.MakeVector` _returnvalue_x _returnvalue_y) (* AxisValue (`self.MovementSpeed`)))))

(event `InputAxis|MovementAxisLeft_Y`
  (params (AxisValue :type "Float (single-precision)"))
  (bind (_returnvalue_x _returnvalue_y) (`KismetMathLibrary.BreakVector` (`SceneComponent.GetForwardVector` (`self.Camera`))))
  ;[1 1 1] Advanced Locomotion
  (if (not (== AxisValue 0.0))
    (`self.AddMovementInput` (`KismetMathLibrary.MakeVector` _returnvalue_x _returnvalue_y) (* AxisValue (`self.MovementSpeed`)))))

(fn `UserConstructionScript`
  (bind _output_get (set `self.IKBody` (`self.IKBody`)))
  (set `IKBodyComponent.Body` (`self.SkeletalMesh`) _output_get)
  (set `IKBodyComponent.Camera` (`self.Camera`) (`self.IKBody`))
  (set `IKBodyComponent.LeftController` (`self.MotionControllerLeft`) (`self.IKBody`))
  (set `IKBodyComponent.RightController` (`self.MotionControllerRight`) (`self.IKBody`)))